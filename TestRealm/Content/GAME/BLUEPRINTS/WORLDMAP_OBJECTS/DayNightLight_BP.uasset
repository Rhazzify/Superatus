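; World map light actor that drives the day/night look and advances the game's time of day.
; On BeginPlay it binds to the GameInfoInstance DayNightCycle event.
; Each event recolors the light by the current TimeOfDay and steps it through four phases, also changing intensity in the last two.
; The final phase resets TimeOfDay, increments Days and calls ShowWorldEvent on the game instance.
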(event Custom|DayNIghtCycle
  (bind _lightcomponent (Variables|Default|GetLightComponent))
  (bind _gameinstance (Variables|Default|GetGameInstance))
  (bind _gameinstance_2 (Variables|Default|GetGameInstance))
  (bind _lightcomponent_2 (Variables|Default|GetLightComponent))
  (switch int (Variables|/Game/GAME/BLUEPRINTS/GAMEINFO/GameInfoInstance.GameInfoInstance_C|GetTimeOfDay (Variables|Default|GetGameInstance))
    (:0
      (Rendering|Components|Light|SetLightColor (Variables|Default|GetLightComponent) "(R=1.000000,G=0.796003,B=0.071455,A=1.000000)" true)
      (bind _result (Math|Integer|IncrementInt (Variables|/Game/GAME/BLUEPRINTS/GAMEINFO/GameInfoInstance.GameInfoInstance_C|GetTimeOfDay _gameinstance) :!label _label)
        (:%20%20
          (Variables|/Game/GAME/BLUEPRINTS/GAMEINFO/GameInfoInstance.GameInfoInstance_C|SetTimeOfDay _gameinstance _result))))
    (:1
      (Rendering|Components|Light|SetLightColor (Variables|Default|GetLightComponent) "(R=1.000000,G=0.181751,B=0.000000,A=1.000000)" true)
      (goto _label))
    (:2
      (Rendering|Components|Light|SetLightColor _lightcomponent_2 "(R=0.000000,G=0.102115,B=0.239583,A=1.000000)" true)
      (Rendering|Components|Light|SetIntensity _lightcomponent_2 5.0)
      (goto _label))
    (:3
      (Rendering|Components|Light|SetLightColor _lightcomponent "(R=1.000000,G=0.967098,B=0.957051,A=1.000000)" true)
      (Rendering|Components|Light|SetIntensity _lightcomponent 1e+01)
      (Variables|/Game/GAME/BLUEPRINTS/GAMEINFO/GameInfoInstance.GameInfoInstance_C|SetTimeOfDay _gameinstance_2 0)
      (bind _result_2 (Math|Integer|IncrementInt (Variables|/Game/GAME/BLUEPRINTS/GAMEINFO/GameInfoInstance.GameInfoInstance_C|GetDays _gameinstance_2))
        (:%20%20
          (Variables|/Game/GAME/BLUEPRINTS/GAMEINFO/GameInfoInstance.GameInfoInstance_C|SetDays _gameinstance_2 _result_2)
          (Default|ShowWorldEvent _gameinstance_2))))))

(event EventBeginPlay
  (bind _asgame_info_instance (Utilities|Casting|CastToGameInfoInstance (Game|GetGameInstance)))
  (bind _output_get (Variables|Default|SetGameInstance _asgame_info_instance))
  (EventDispatchers|BindEventtoDayNightCycle _output_get (delegate Custom|DayNIghtCycle)))

(fn ConstructionScript)
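; GameInfoInstance is the central UI manager that opens and closes zone upgrade, quest and event screens, plus minimap, crafting and popup widgets.
; Show events lazily create and cache each widget before adding it to the viewport; Remove events detach it, with IsValid checks that guard nothing.
; Run functions open world, forage, explore and fishing widgets.
; World events favour WorldEvent01 four-to-one over the monster event, leaving WorldEvent03 unreachable.
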(event Custom|Show%20Resource
  ;[1 1 1] ResourceIndicator
  (Utilities|IsValid (Variables|Resource|GetResourceIndicatorWB)
    (:Is%20Valid
      _)
    (:Is%20Not%20Valid
      (bind _returnvalue (UserInterface|CreateWidget "/Game/GAME/BLUEPRINTS/WIDGETS/HUD/ResourceIndicator.ResourceIndicator_C" (Game|GetPlayerController 0)))
      (bind _output_get (Variables|Resource|SetResourceIndicatorWB _returnvalue))))
  (UserInterface|Viewport|AddtoViewport _output_get 0))

(event Custom|Show%20sleeping
  ;[1 1 1] Sleeping event
  (Utilities|IsValid (stale _returnvalue)
    (:Is%20Valid
      _)
    (:Is%20Not%20Valid
      (bind _returnvalue (UserInterface|CreateWidget "/Game/GAME/BLUEPRINTS/WIDGETS/HUD/Sleeping.Sleeping_C" (Game|GetPlayerController 0)))))
  (UserInterface|Viewport|AddtoViewport _returnvalue 0))

(event Custom|Show%20NotEnoughEnergy
  ;[1 1 1] Not Enough energy PopUp
  (Utilities|IsValid (Variables|PopUps|GetNotEnoughEnergyWB)
    (:Is%20Valid
      _)
    (:Is%20Not%20Valid
      (bind _returnvalue (UserInterface|CreateWidget "/Game/GAME/BLUEPRINTS/WIDGETS/HUD/NotEnoughEnergy.NotEnoughEnergy_C" (Game|GetPlayerController 0)))
      (bind _output_get (Variables|PopUps|SetNotEnoughEnergyWB _returnvalue))))
  (UserInterface|Viewport|AddtoViewport _output_get 0))

(event Custom|Show%20Explore
  (CallFunction|RunExplore))

(event Custom|Remove%20NotEnoughEnergy
  (bind _notenoughenergywb (Variables|PopUps|GetNotEnoughEnergyWB))
  ;[1 1 1] Not Enough energy PopUp
  (Utilities|IsValid _notenoughenergywb
    (:Is%20Valid
      _)
    (:Is%20Not%20Valid
      _))
  (Widget|RemovefromParent _notenoughenergywb))

(event Custom|Show%20Monster
  ;[1 1 1] Monster event
  (Utilities|IsValid (stale _returnvalue)
    (:Is%20Valid
      _)
    (:Is%20Not%20Valid
      (bind _returnvalue (UserInterface|CreateWidget "/Game/GAME/BLUEPRINTS/WIDGETS/WORLD_AREAS/TEMPLATE_EVENTS/MonsterEV1.MonsterEV1_C" (Game|GetPlayerController 0)))))
  (UserInterface|Viewport|AddtoViewport _returnvalue 0))

(event Custom|Show%20Jungle%20Events
  ;[0.215 0 1 1 30] ZONE EVENTS
  ;;[1 1 1] Jungle Events
  (Utilities|IsValid (Variables|WorldMapCHoices|GetJungle%20Choice)
    (:Is%20Valid
      _)
    (:Is%20Not%20Valid
      (bind _returnvalue (UserInterface|CreateWidget "/Game/GAME/BLUEPRINTS/WIDGETS/WORLD_AREAS/JUNGLE/JungleChoices_WB.JungleChoices_WB_C" (Game|GetPlayerController 0)))
      (bind _output_get (Variables|WorldMapCHoices|SetJungle%20Choice _returnvalue))))
  (UserInterface|Viewport|AddtoViewport _output_get 0))

(event Custom|Remove%20Jungle%20Events
  (bind _jungle_choice (Variables|WorldMapCHoices|GetJungle%20Choice))
  ;[0.215 0 1 1 30] ZONE EVENTS
  ;;[1 1 1] Jungle Events
  (Utilities|IsValid _jungle_choice
    (:Is%20Valid
      _)
    (:Is%20Not%20Valid
      _))
  (Widget|RemovefromParent _jungle_choice))

(event Custom|Show%20Village%20Events
  ;[0.215 0 1 1 30] ZONE EVENTS
  ;;[1 1 1] Village Events
  (Utilities|IsValid (Variables|WorldMapCHoices|GetVillage%20Choice)
    (:Is%20Valid
      _)
    (:Is%20Not%20Valid
      (bind _returnvalue (UserInterface|CreateWidget "/Game/GAME/BLUEPRINTS/WIDGETS/WORLD_AREAS/VILLAGE/VillageChoices_WB.VillageChoices_WB_C" (Game|GetPlayerController 0)))
      (bind _output_get (Variables|WorldMapCHoices|SetVillage%20Choice _returnvalue))))
  (UserInterface|Viewport|AddtoViewport _output_get 0))

(event Custom|Remove%20Village%20Events
  (bind _village_choice (Variables|WorldMapCHoices|GetVillage%20Choice))
  ;[0.215 0 1 1 30] ZONE EVENTS
  ;;[1 1 1] Village Events
  (Utilities|IsValid _village_choice
    (:Is%20Valid
      _)
    (:Is%20Not%20Valid
      _))
  (Widget|RemovefromParent _village_choice))

(event Custom|Show%20Desert%20Events
  ;[0.215 0 1 1 30] ZONE EVENTS
  ;;[1 1 1] Desert Events
  (Utilities|IsValid (Variables|WorldMapCHoices|GetDesert%20Choice)
    (:Is%20Valid
      _)
    (:Is%20Not%20Valid
      (bind _returnvalue (UserInterface|CreateWidget "/Game/GAME/BLUEPRINTS/WIDGETS/WORLD_AREAS/DESERT/DesertChoices_WB.DesertChoices_WB_C" (Game|GetPlayerController 0)))
      (bind _output_get (Variables|WorldMapCHoices|SetDesert%20Choice _returnvalue))))
  (UserInterface|Viewport|AddtoViewport _output_get 0))

(event Custom|Remove%20Desert%20Events
  (bind _desert_choice (Variables|WorldMapCHoices|GetDesert%20Choice))
  ;[0.215 0 1 1 30] ZONE EVENTS
  ;;[1 1 1] Desert Events
  (Utilities|IsValid _desert_choice
    (:Is%20Valid
      _)
    (:Is%20Not%20Valid
      _))
  (Widget|RemovefromParent _desert_choice))

(event Custom|Show%20Lake%20Events
  ;[0.215 0 1 1 30] ZONE EVENTS
  ;;[1 1 1] Lake Events
  (Utilities|IsValid (Variables|WorldMapCHoices|GetLake%20Choice)
    (:Is%20Valid
      _)
    (:Is%20Not%20Valid
      (bind _returnvalue (UserInterface|CreateWidget "/Game/GAME/BLUEPRINTS/WIDGETS/WORLD_AREAS/LAKE/LakeChoices_WB.LakeChoices_WB_C" (Game|GetPlayerController 0)))
      (bind _output_get (Variables|WorldMapCHoices|SetLake%20Choice _returnvalue))))
  (UserInterface|Viewport|AddtoViewport _output_get 0))

(event Custom|Remove%20Lake%20Events
  (bind _lake_choice (Variables|WorldMapCHoices|GetLake%20Choice))
  ;[0.215 0 1 1 30] ZONE EVENTS
  ;;[1 1 1] Lake Events
  (Utilities|IsValid _lake_choice
    (:Is%20Valid
      _)
    (:Is%20Not%20Valid
      _))
  (Widget|RemovefromParent _lake_choice))

(event Custom|Show%20Beach%20Events
  ;[0.215 0 1 1 30] ZONE EVENTS
  ;;[1 1 1] Beach Events
  (Utilities|IsValid (Variables|WorldMapCHoices|GetBeach%20Choice)
    (:Is%20Valid
      _)
    (:Is%20Not%20Valid
      (bind _returnvalue (UserInterface|CreateWidget "/Game/GAME/BLUEPRINTS/WIDGETS/WORLD_AREAS/BEACH/BeachChoices_WB.BeachChoices_WB_C" (Game|GetPlayerController 0)))
      (bind _output_get (Variables|WorldMapCHoices|SetBeach%20Choice _returnvalue))))
  (UserInterface|Viewport|AddtoViewport _output_get 0))

(event Custom|Remove%20Beach%20Events
  (bind _beach_choice (Variables|WorldMapCHoices|GetBeach%20Choice))
  ;[0.215 0 1 1 30] ZONE EVENTS
  ;;[1 1 1] Beach Events
  (Utilities|IsValid _beach_choice
    (:Is%20Valid
      _)
    (:Is%20Not%20Valid
      _))
  (Widget|RemovefromParent _beach_choice))

(event Custom|Show%20Mountain%20Events
  ;[0.215 0 1 1 30] ZONE EVENTS
  ;;[1 1 1] Mountain Events
  (Utilities|IsValid (Variables|WorldMapCHoices|GetMountain%20Choices)
    (:Is%20Valid
      _)
    (:Is%20Not%20Valid
      (bind _returnvalue (UserInterface|CreateWidget "/Game/GAME/BLUEPRINTS/WIDGETS/WORLD_AREAS/MOUNTAIN/MountainChoices_WB.MountainChoices_WB_C" (Game|GetPlayerController 0)))
      (bind _output_get (Variables|WorldMapCHoices|SetMountain%20Choices _returnvalue))))
  (UserInterface|Viewport|AddtoViewport _output_get 0))

(event Custom|Remove%20Mountain%20Events
  (bind _mountain_choices (Variables|WorldMapCHoices|GetMountain%20Choices))
  ;[0.215 0 1 1 30] ZONE EVENTS
  ;;[1 1 1] Mountain Events
  (Utilities|IsValid _mountain_choices
    (:Is%20Valid
      _)
    (:Is%20Not%20Valid
      _))
  (Widget|RemovefromParent _mountain_choices))

(event Custom|Show%20Forest%20Events
  ;[0.215 0 1 1 30] ZONE EVENTS
  ;;[1 1 1] Forest Events
  (Utilities|IsValid (Variables|WorldMapCHoices|GetForest%20Choice)
    (:Is%20Valid
      _)
    (:Is%20Not%20Valid
      (bind _returnvalue (UserInterface|CreateWidget "/Game/GAME/BLUEPRINTS/WIDGETS/WORLD_AREAS/FOREST/ForestChoices_WB.ForestChoices_WB_C" (Game|GetPlayerController 0)))
      (bind _output_get (Variables|WorldMapCHoices|SetForest%20Choice _returnvalue))))
  (UserInterface|Viewport|AddtoViewport _output_get 0))

(event Custom|Remove%20Forest%20Events
  (bind _forest_choice (Variables|WorldMapCHoices|GetForest%20Choice))
  ;[0.215 0 1 1 30] ZONE EVENTS
  ;;[1 1 1] Forest Events
  (Utilities|IsValid _forest_choice
    (:Is%20Valid
      _)
    (:Is%20Not%20Valid
      _))
  (Widget|RemovefromParent _forest_choice))

(event Custom|Remove%20Monster
  ;[1 1 1] Monster event
  (Utilities|IsValid (stale Custom|Show%20Monster _returnvalue)
    (:Is%20Valid
      _)
    (:Is%20Not%20Valid
      _))
  (Widget|RemovefromParent (stale Custom|Show%20Monster _returnvalue)))

(event Custom|Show%20Crafting
  ;[1 1 1] Show Crafting
  (Utilities|IsValid (stale _returnvalue)
    (:Is%20Valid
      _)
    (:Is%20Not%20Valid
      (bind _returnvalue (UserInterface|CreateWidget "/Game/GAME/BLUEPRINTS/WIDGETS/WORLD_AREAS/VILLAGE/UPGRADE_VILLAGE/CraftingVillage.CraftingVillage_C" (Game|GetPlayerController 0)))))
  (UserInterface|Viewport|AddtoViewport _returnvalue 0))

(event Custom|Show%20DesertUpgrades
  ;[0 1 0.0563 1 30] ZONE UPGRADES
  ;;[1 1 1] Desert upgrades
  (Utilities|IsValid (stale _returnvalue)
    (:Is%20Valid
      _)
    (:Is%20Not%20Valid
      (bind _returnvalue (UserInterface|CreateWidget "/Game/GAME/BLUEPRINTS/WIDGETS/WORLD_AREAS/DESERT/UPGRADES_DESERT/UpgradeDesert.UpgradeDesert_C" (Game|GetPlayerController 0)))))
  (UserInterface|Viewport|AddtoViewport _returnvalue 0))

(event Custom|Remove%20DesertUpgrades
  ;[0 1 0.0563 1 30] ZONE UPGRADES
  ;;[1 1 1] Desert upgrades
  (Utilities|IsValid (stale Custom|Show%20DesertUpgrades _returnvalue)
    (:Is%20Valid
      _)
    (:Is%20Not%20Valid
      _))
  (Widget|RemovefromParent (stale Custom|Show%20DesertUpgrades _returnvalue)))

(event Custom|Show%20RequirementNotMet
  ;[1 1 1] Not Enough energy PopUp
  (Utilities|IsValid (stale _output_get)
    (:Is%20Valid
      _)
    (:Is%20Not%20Valid
      (bind _returnvalue (UserInterface|CreateWidget "/Game/GAME/BLUEPRINTS/WIDGETS/HUD/RequirementsNotMet.RequirementsNotMet_C" (Game|GetPlayerController 0)))
      (bind _output_get (Variables|PopUps|SetRequirementsNotMet _returnvalue))))
  (UserInterface|Viewport|AddtoViewport _output_get 0))

(event Custom|Remove%20RequirementNotMet
  ;[1 1 1] Not Enough energy PopUp
  (Utilities|IsValid (stale Custom|Show%20RequirementNotMet _output_get)
    (:Is%20Valid
      _)
    (:Is%20Not%20Valid
      _))
  (Widget|RemovefromParent (stale Custom|Show%20RequirementNotMet _output_get)))

(event Custom|Show%20JungleQuest
  ;[1 0.9591 0.1563 1 30] ZONE QUESTS
  ;;[1 1 1] Jungle quests
  (Utilities|IsValid (stale _returnvalue)
    (:Is%20Valid
      _)
    (:Is%20Not%20Valid
      (bind _returnvalue (UserInterface|CreateWidget "/Game/GAME/BLUEPRINTS/WIDGETS/WORLD_AREAS/JUNGLE/QUEST_JUNGLE/JungleQuest.JungleQuest_C" (Game|GetPlayerController 0)))))
  (UserInterface|Viewport|AddtoViewport _returnvalue 0))

(event Custom|Remove%20JungleQuest
  ;[1 0.9591 0.1563 1 30] ZONE QUESTS
  ;;[1 1 1] Jungle quests
  (Utilities|IsValid (stale Custom|Show%20JungleQuest _returnvalue)
    (:Is%20Valid
      _)
    (:Is%20Not%20Valid
      _))
  (Widget|RemovefromParent (stale Custom|Show%20JungleQuest _returnvalue)))

(event Custom|Show%20VillageQuest
  ;[1 0.9591 0.1563 1 30] ZONE QUESTS
  ;;[1 1 1] Village quests
  (Utilities|IsValid (stale _returnvalue)
    (:Is%20Valid
      _)
    (:Is%20Not%20Valid
      (bind _returnvalue (UserInterface|CreateWidget "/Game/GAME/BLUEPRINTS/WIDGETS/WORLD_AREAS/VILLAGE/QUEST_VILLAGE/VillageQuest.VillageQuest_C" (Game|GetPlayerController 0)))))
  (UserInterface|Viewport|AddtoViewport _returnvalue 0))

(event Custom|Remove%20VillageQuest
  ;[1 0.9591 0.1563 1 30] ZONE QUESTS
  ;;[1 1 1] Village quests
  (Utilities|IsValid (stale Custom|Show%20VillageQuest _returnvalue)
    (:Is%20Valid
      _)
    (:Is%20Not%20Valid
      _))
  (Widget|RemovefromParent (stale Custom|Show%20VillageQuest _returnvalue)))

(event Custom|Show%20DesertQuest
  ;[1 0.9591 0.1563 1 30] ZONE QUESTS
  ;;[1 1 1] Desert quests
  (Utilities|IsValid (stale _returnvalue)
    (:Is%20Valid
      _)
    (:Is%20Not%20Valid
      (bind _returnvalue (UserInterface|CreateWidget "/Game/GAME/BLUEPRINTS/WIDGETS/WORLD_AREAS/DESERT/QUEST_DESERT/DesertQuest.DesertQuest_C" (Game|GetPlayerController 0)))))
  (UserInterface|Viewport|AddtoViewport _returnvalue 0))

(event Custom|Remove%20DesertQuest
  ;[1 0.9591 0.1563 1 30] ZONE QUESTS
  ;;[1 1 1] Desert quests
  (Utilities|IsValid (stale Custom|Show%20DesertQuest _returnvalue)
    (:Is%20Valid
      _)
    (:Is%20Not%20Valid
      _))
  (Widget|RemovefromParent (stale Custom|Show%20DesertQuest _returnvalue)))

(event Custom|Show%20LakeQuest
  ;[1 0.9591 0.1563 1 30] ZONE QUESTS
  ;;[1 1 1] Lake quests
  (Utilities|IsValid (stale _returnvalue)
    (:Is%20Valid
      _)
    (:Is%20Not%20Valid
      (bind _returnvalue (UserInterface|CreateWidget "/Game/GAME/BLUEPRINTS/WIDGETS/WORLD_AREAS/LAKE/QUEST_LAKE/LakeQuest.LakeQuest_C" (Game|GetPlayerController 0)))))
  (UserInterface|Viewport|AddtoViewport _returnvalue 0))

(event Custom|Remove%20LakeQuest
  ;[1 0.9591 0.1563 1 30] ZONE QUESTS
  ;;[1 1 1] Lake quests
  (Utilities|IsValid (stale Custom|Show%20LakeQuest _returnvalue)
    (:Is%20Valid
      _)
    (:Is%20Not%20Valid
      _))
  (Widget|RemovefromParent (stale Custom|Show%20LakeQuest _returnvalue)))

(event Custom|Show%20BeachQuest
  ;[1 0.9591 0.1563 1 30] ZONE QUESTS
  ;;[1 1 1] Beach quests
  (Utilities|IsValid (stale _returnvalue)
    (:Is%20Valid
      _)
    (:Is%20Not%20Valid
      (bind _returnvalue (UserInterface|CreateWidget "/Game/GAME/BLUEPRINTS/WIDGETS/WORLD_AREAS/BEACH/QUEST_BEACH/BeachQuest.BeachQuest_C" (Game|GetPlayerController 0)))))
  (UserInterface|Viewport|AddtoViewport _returnvalue 0))

(event Custom|Remove%20BeachQuest
  ;[1 0.9591 0.1563 1 30] ZONE QUESTS
  ;;[1 1 1] Beach quests
  (Utilities|IsValid (stale Custom|Show%20BeachQuest _returnvalue)
    (:Is%20Valid
      _)
    (:Is%20Not%20Valid
      _))
  (Widget|RemovefromParent (stale Custom|Show%20BeachQuest _returnvalue)))

(event Custom|Show%20MountainQuest
  ;[1 0.9591 0.1563 1 30] ZONE QUESTS
  ;;[1 1 1] Mountain quests
  (Utilities|IsValid (stale _returnvalue)
    (:Is%20Valid
      _)
    (:Is%20Not%20Valid
      (bind _returnvalue (UserInterface|CreateWidget "/Game/GAME/BLUEPRINTS/WIDGETS/WORLD_AREAS/MOUNTAIN/QUEST_MOUNTAIN/MountainQuest.MountainQuest_C" (Game|GetPlayerController 0)))))
  (UserInterface|Viewport|AddtoViewport _returnvalue 0))

(event Custom|Remove%20MountainQuest
  ;[1 0.9591 0.1563 1 30] ZONE QUESTS
  ;;[1 1 1] Mountain quests
  (Utilities|IsValid (stale Custom|Show%20MountainQuest _returnvalue)
    (:Is%20Valid
      _)
    (:Is%20Not%20Valid
      _))
  (Widget|RemovefromParent (stale Custom|Show%20MountainQuest _returnvalue)))

(event Custom|Show%20ForestQuests
  ;[1 0.9591 0.1563 1 30] ZONE QUESTS
  ;;[1 1 1] Forest quests
  (Utilities|IsValid (stale _returnvalue)
    (:Is%20Valid
      _)
    (:Is%20Not%20Valid
      (bind _returnvalue (UserInterface|CreateWidget "/Game/GAME/BLUEPRINTS/WIDGETS/WORLD_AREAS/FOREST/QUEST_FOREST/ForestQuest.ForestQuest_C" (Game|GetPlayerController 0)))))
  (UserInterface|Viewport|AddtoViewport _returnvalue 0))

(event Custom|Remove%20ForestQuests
  ;[1 0.9591 0.1563 1 30] ZONE QUESTS
  ;;[1 1 1] Forest quests
  (Utilities|IsValid (stale Custom|Show%20ForestQuests _returnvalue)
    (:Is%20Valid
      _)
    (:Is%20Not%20Valid
      _))
  (Widget|RemovefromParent (stale Custom|Show%20ForestQuests _returnvalue)))

(event Custom|Remove%20sleeping
  ;[1 1 1] Sleeping event
  (Utilities|IsValid (stale Custom|Show%20sleeping _returnvalue)
    (:Is%20Valid
      _)
    (:Is%20Not%20Valid
      _))
  (Widget|RemovefromParent (stale Custom|Show%20sleeping _returnvalue)))

(event Custom|Show%20LakeUpgrades
  ;[0 1 0.0563 1 30] ZONE UPGRADES
  ;;[1 1 1] Lake upgrades
  (Utilities|IsValid (stale _returnvalue)
    (:Is%20Valid
      _)
    (:Is%20Not%20Valid
      (bind _returnvalue (UserInterface|CreateWidget "/Game/GAME/BLUEPRINTS/WIDGETS/WORLD_AREAS/LAKE/UPGRADE_LAKE/UpgradeLake.UpgradeLake_C" (Game|GetPlayerController 0)))))
  (UserInterface|Viewport|AddtoViewport _returnvalue 0))

(event Custom|Remove%20LakeUpgrades
  ;[0 1 0.0563 1 30] ZONE UPGRADES
  ;;[1 1 1] Lake upgrades
  (Utilities|IsValid (stale Custom|Show%20LakeUpgrades _returnvalue)
    (:Is%20Valid
      _)
    (:Is%20Not%20Valid
      _))
  (Widget|RemovefromParent (stale Custom|Show%20LakeUpgrades _returnvalue)))

(event Custom|Show%20BeachUpgrades
  ;[0 1 0.0563 1 30] ZONE UPGRADES
  ;;[1 1 1] Beach upgrades
  (Utilities|IsValid (stale _returnvalue)
    (:Is%20Valid
      _)
    (:Is%20Not%20Valid
      (bind _returnvalue (UserInterface|CreateWidget "/Game/GAME/BLUEPRINTS/WIDGETS/WORLD_AREAS/BEACH/UPGRADE_BEACH/UpgradeBeach.UpgradeBeach_C" (Game|GetPlayerController 0)))))
  (UserInterface|Viewport|AddtoViewport _returnvalue 0))

(event Custom|Remove%20BeachUpgrades
  ;[0 1 0.0563 1 30] ZONE UPGRADES
  ;;[1 1 1] Beach upgrades
  (Utilities|IsValid (stale Custom|Show%20BeachUpgrades _returnvalue)
    (:Is%20Valid
      _)
    (:Is%20Not%20Valid
      _))
  (Widget|RemovefromParent (stale Custom|Show%20BeachUpgrades _returnvalue)))

(event Custom|Show%20MountainUpgrades
  ;[0 1 0.0563 1 30] ZONE UPGRADES
  ;;[1 1 1] Mountain upgrades
  (Utilities|IsValid (stale _returnvalue)
    (:Is%20Valid
      _)
    (:Is%20Not%20Valid
      (bind _returnvalue (UserInterface|CreateWidget "/Game/GAME/BLUEPRINTS/WIDGETS/WORLD_AREAS/MOUNTAIN/UPGRADE_MOUNTAIN/UpgradeMountain.UpgradeMountain_C" (Game|GetPlayerController 0)))))
  (UserInterface|Viewport|AddtoViewport _returnvalue 0))

(event Custom|Remove%20MountainUpgrades
  ;[0 1 0.0563 1 30] ZONE UPGRADES
  ;;[1 1 1] Mountain upgrades
  (Utilities|IsValid (stale Custom|Show%20MountainUpgrades _returnvalue)
    (:Is%20Valid
      _)
    (:Is%20Not%20Valid
      _))
  (Widget|RemovefromParent (stale Custom|Show%20MountainUpgrades _returnvalue)))

(event Custom|Show%20JungleUpgrades
  ;[0 1 0.0563 1 30] ZONE UPGRADES
  ;;[1 1 1] Jungle upgrades
  (Utilities|IsValid (stale _returnvalue)
    (:Is%20Valid
      _)
    (:Is%20Not%20Valid
      (bind _returnvalue (UserInterface|CreateWidget "/Game/GAME/BLUEPRINTS/WIDGETS/WORLD_AREAS/JUNGLE/UPGRADE_JUNGLE/UpgradeJungle.UpgradeJungle_C" (Game|GetPlayerController 0)))))
  (UserInterface|Viewport|AddtoViewport _returnvalue 0))

(event Custom|Show%20WorldEvent
  (CallFunction|RunWorldEvents))

(event Custom|Remove%20JungleUpgrades
  ;[0 1 0.0563 1 30] ZONE UPGRADES
  ;;[1 1 1] Jungle upgrades
  (Utilities|IsValid (stale Custom|Show%20JungleUpgrades _returnvalue)
    (:Is%20Valid
      _)
    (:Is%20Not%20Valid
      _))
  (Widget|RemovefromParent (stale Custom|Show%20JungleUpgrades _returnvalue)))

(event Custom|Show%20ForestUpgrades
  ;[0 1 0.0563 1 30] ZONE UPGRADES
  ;;[1 1 1] Forest upgrades
  (Utilities|IsValid (stale _returnvalue)
    (:Is%20Valid
      _)
    (:Is%20Not%20Valid
      (bind _returnvalue (UserInterface|CreateWidget "/Game/GAME/BLUEPRINTS/WIDGETS/WORLD_AREAS/FOREST/UPGRADE_FOREST/UpgradeForest.UpgradeForest_C" (Game|GetPlayerController 0)))))
  (UserInterface|Viewport|AddtoViewport _returnvalue 0))

(event Custom|ShowMiniMap
  ;[1 1 1] Show Minimap
  (Utilities|IsValid (Variables|Default|GetMinimapWB)
    (:Is%20Valid
      _)
    (:Is%20Not%20Valid
      (bind _returnvalue (UserInterface|CreateWidget "/Game/GAME/BLUEPRINTS/WIDGETS/HUD/MiniMapMovement.MiniMapMovement_C" (Game|GetPlayerController 0)))
      (bind _output_get (Variables|Default|SetMinimapWB _returnvalue))))
  (UserInterface|Viewport|AddtoViewport _output_get 0))

(event Custom|Remove%20ForestUpgrades
  ;[0 1 0.0563 1 30] ZONE UPGRADES
  ;;[1 1 1] Forest upgrades
  (Utilities|IsValid (stale Custom|Show%20ForestUpgrades _returnvalue)
    (:Is%20Valid
      _)
    (:Is%20Not%20Valid
      _))
  (Widget|RemovefromParent (stale Custom|Show%20ForestUpgrades _returnvalue)))

(event Custom|RemoveMiniMap
  ;[1 1 1] Show Minimap
  (Utilities|IsValid (Variables|Default|GetMinimapWB)
    (:Is%20Valid
      _)
    (:Is%20Not%20Valid
      _))
  (Widget|RemovefromParent (Variables|Default|GetMinimapWB)))

(event Custom|Show%20ForageTree
  (CallFunction|RunForageTree))

(event Custom|Show%20VillageUpgrades
  ;[0 1 0.0563 1 30] ZONE UPGRADES
  ;;[1 1 1] Village upgrades
  (Utilities|IsValid (stale _returnvalue)
    (:Is%20Valid
      _)
    (:Is%20Not%20Valid
      (bind _returnvalue (UserInterface|CreateWidget "/Game/GAME/BLUEPRINTS/WIDGETS/WORLD_AREAS/VILLAGE/UPGRADE_VILLAGE/UpgradeVillage.UpgradeVillage_C" (Game|GetPlayerController 0)))))
  (UserInterface|Viewport|AddtoViewport _returnvalue 0))

(event Custom|Remove%20VillageUpgrades
  ;[0 1 0.0563 1 30] ZONE UPGRADES
  ;;[1 1 1] Village upgrades
  (Utilities|IsValid (stale Custom|Show%20VillageUpgrades _returnvalue)
    (:Is%20Valid
      _)
    (:Is%20Not%20Valid
      _))
  (Widget|RemovefromParent (stale Custom|Show%20VillageUpgrades _returnvalue)))

(fn RunWorldEvents
  (switch int (Math|Random|RandomInteger 5)
    (:0
      (Utilities|IsValid (Variables|Default|GetWorldEvent01) :!label _label
        (:Is%20Valid
          _)
        (:Is%20Not%20Valid
          (bind _returnvalue (UserInterface|CreateWidget "/Game/GAME/BLUEPRINTS/WIDGETS/WORLD_EVENTS/WorldEvent01_WB.WorldEvent01_WB_C" (Game|GetPlayerController 0)))
          (bind _output_get (Variables|Default|SetWorldEvent01 _returnvalue))))
      (UserInterface|Viewport|AddtoViewport _output_get 0))
    (:1
      (goto _label))
    (:2
      (Utilities|IsValid (Variables|Default|GetWorldEvent02)
        (:Is%20Valid
          _)
        (:Is%20Not%20Valid
          (bind _returnvalue_2 (UserInterface|CreateWidget "/Game/GAME/BLUEPRINTS/WIDGETS/WORLD_EVENTS/WorldEvent02_MONSTER.WorldEvent02_MONSTER_C" (Game|GetPlayerController 0)))
          (bind _output_get_2 (Variables|Default|SetWorldEvent02 _returnvalue_2))))
      (UserInterface|Viewport|AddtoViewport _output_get_2 0))
    (:3
      (goto _label))
    (:4
      (goto _label))))

(fn RunForageTree
  (switch int (Math|Random|RandomInteger 3)
    (:0
      (Utilities|IsValid (stale _returnvalue)
        (:Is%20Valid
          _)
        (:Is%20Not%20Valid
          (bind _returnvalue (UserInterface|CreateWidget "/Game/GAME/BLUEPRINTS/WIDGETS/WORLD_AREAS/TEMPLATE_EVENTS/ForageEV01.ForageEV01_C" (Game|GetPlayerController 0)))))
      (UserInterface|Viewport|AddtoViewport _returnvalue 0))
    (:1
      (Utilities|IsValid (stale _returnvalue_2)
        (:Is%20Valid
          _)
        (:Is%20Not%20Valid
          (bind _returnvalue_2 (UserInterface|CreateWidget "/Game/GAME/BLUEPRINTS/WIDGETS/WORLD_AREAS/TEMPLATE_EVENTS/ForageEV02.ForageEV02_C" (Game|GetPlayerController 0)))))
      (UserInterface|Viewport|AddtoViewport _returnvalue_2 0))
    (:2
      (Utilities|IsValid (stale _returnvalue_3)
        (:Is%20Valid
          _)
        (:Is%20Not%20Valid
          (bind _returnvalue_3 (UserInterface|CreateWidget "/Game/GAME/BLUEPRINTS/WIDGETS/WORLD_AREAS/TEMPLATE_EVENTS/ForageEV03.ForageEV03_C" (Game|GetPlayerController 0)))))
      (UserInterface|Viewport|AddtoViewport _returnvalue_3 0))))

(fn RunExplore
  (Utilities|IsValid (stale _returnvalue)
    (:Is%20Valid
      _)
    (:Is%20Not%20Valid
      (bind _returnvalue (UserInterface|CreateWidget "/Game/GAME/BLUEPRINTS/WIDGETS/WORLD_AREAS/TEMPLATE_EVENTS/ExploreEvent01_WB.ExploreEvent01_WB_C" (Game|GetPlayerController 0)))))
  (UserInterface|Viewport|AddtoViewport _returnvalue 0))

(fn RunFishingLake
  (Utilities|IsValid (stale _returnvalue)
    (:Is%20Valid
      _)
    (:Is%20Not%20Valid
      (bind _returnvalue (UserInterface|CreateWidget "/Game/GAME/BLUEPRINTS/WIDGETS/WORLD_AREAS/LAKE/FISHING_LAKE/RandomFishingLake.RandomFishingLake_C" (Game|GetPlayerController 0)))))
  (Default|RandomizeLakeFishing _returnvalue)
  (UserInterface|Viewport|AddtoViewport _returnvalue 0))

(fn RunExploreBeach
  (switch int 0))
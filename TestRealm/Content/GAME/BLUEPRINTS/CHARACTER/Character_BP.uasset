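; Character Blueprint that walks its pawn to one of seven map locations: Village, Jungle, Desert, Lake, Mountain, Forest or Beach.
; On BeginPlay it casts the game instance to GameInfoInstance and binds a custom event to each of its move-to-location dispatchers.
; Each event calls AI MoveTo on the controlled pawn with a hardcoded world coordinate for that location.
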(event Custom|CharacterMoveBeach
  ;[1 1 1] Move to Beach
  (AI|AIMoveTo (Pawn|GetControlledPawn (Pawn|GetController)) "-796.000000,-14.000000,-1.000000" 0 5.0 false))

(event Custom|CharacterMoveLake
  ;[1 1 1] Move to Lake
  (AI|AIMoveTo (Pawn|GetControlledPawn (Pawn|GetController)) "-739.000000,-843.000000,12.000000" 0 5.0 false))

(event Custom|CharacterMoveJungle
  ;[1 1 1] Move to Jungle
  (AI|AIMoveTo (Pawn|GetControlledPawn (Pawn|GetController)) "730.000000,-840.000000,24.000000" 0 5.0 false))

(event Custom|CharacterMoveDesert
  ;[1 1 1] Move to Desert
  (AI|AIMoveTo (Pawn|GetControlledPawn (Pawn|GetController)) "-762.000000,782.000000,6.000000" 0 5.0 false))

(event Custom|CharacterMoveVillage
  ;[1 1 1] Move to Village
  (AI|AIMoveTo (Pawn|GetControlledPawn (Pawn|GetController)) "742.000000,779.000000,21.000000" 0 5.0 false))

(event Custom|CharacterMoveMountain
  ;[1 1 1] Move to Mountain
  (AI|AIMoveTo (Pawn|GetControlledPawn (Pawn|GetController)) "761.000000,30.000000,3.000000" 0 5.0 false))

(event Custom|CharacterMoveForest
  ;[1 1 1] Move to Forest
  (AI|AIMoveTo (Pawn|GetControlledPawn (Pawn|GetController)) "-68.000000,791.000000,3.000000" 0 5.0 false))

(event EventBeginPlay
  (bind _asgame_info_instance (Utilities|Casting|CastToGameInfoInstance (Game|GetGameInstance)))
  (EventDispatchers|BindEventtoMovetoVillage _asgame_info_instance (delegate Custom|CharacterMoveVillage))
  (EventDispatchers|BindEventtoMovetoJungle _asgame_info_instance (delegate Custom|CharacterMoveJungle))
  (EventDispatchers|BindEventtoMovetoDesert _asgame_info_instance (delegate Custom|CharacterMoveDesert))
  (EventDispatchers|BindEventtoMovetoLake _asgame_info_instance (delegate Custom|CharacterMoveLake))
  (EventDispatchers|BindEventtoMovetoMountain _asgame_info_instance (delegate Custom|CharacterMoveMountain))
  (EventDispatchers|BindEventtoMovetoForest _asgame_info_instance (delegate Custom|CharacterMoveForest))
  (EventDispatchers|BindEventtoMovetoBeach _asgame_info_instance (delegate Custom|CharacterMoveBeach)))

(fn ConstructionScript)